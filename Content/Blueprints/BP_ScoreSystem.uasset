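; BP_ScoreSystem is the run scoring Blueprint, awarding points for time survived and triggering the player's win.
; On run start it finds the BP_Player, stores the given HUD and starts a looping timer that increments the score and pushes it to the HUD.
; Once the score nears one hundred, each tick calls OnGameWon on the player until the run-ended event clears the timer.
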(event `OnRunStarted`
  (params (PlayerHud :type "/Game/UI/PlayerUI Object Reference"))
  (`|ExecutionSequence`
    (:`then_0`
      (bind _returnvalue (`GameplayStatics.GetActorOfClass` "/Game/Blueprints/BP_Player.BP_Player_C"))
      (`/Engine/EditorBlueprintResources/StandardMacros.IsValid` _returnvalue
        (:`Is Valid`
          (set `self.Player` _returnvalue))))
    (:`then_1`
      (set `self.PlayerHudRef` PlayerHud)
      (bind _returnvalue_2 (`KismetSystemLibrary.K2_SetTimerDelegate` (delegate `CalculateScore`) 0.1 true))
      (set `self.ScoreHandle` _returnvalue_2))))

(event `CalculateScore`
  (bind _returnvalue (+ (`self.Score`) 1))
  (bind _output_get (set `self.Score` _returnvalue))
  (`/Game/UI/PlayerUI.OnScoreChanged` (`self.PlayerHudRef`) _output_get)
  (if (>= _returnvalue 100)
    (`/Game/Blueprints/BP_Player.OnGameWon` (`self.Player`))))

(event `OnRunEnded`
  (`KismetSystemLibrary.K2_ClearAndInvalidateTimerHandle` (`self.ScoreHandle`)))

(fn `UserConstructionScript`)